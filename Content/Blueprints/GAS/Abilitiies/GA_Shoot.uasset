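; Gameplay ability that fires a shot for the laser tank or an enemy in a Space Invaders game.
; It spawns a random shot type from the shooter's gun data at its offset texel position, passing a GE_MakeDamage effect spec.
; The shot gets vertical texel velocity from its class speed and gun direction.
; Activation requires the tank's CanShot check, while enemies always qualify because SwarmMind chooses who shoots.
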(event Ability|EventActivateAbility
  (bind _returnvalue (Ability|GetAvatarActorfromActorInfo))
  (bind _asbp_laser_tank (Utilities|Casting|CastToBP_LaserTank _returnvalue)
    (:then
      (Variables|Variables|SetASC (Class|LaserTank|GetCustomAbilitySystemComponent _asbp_laser_tank))
      (Variables|Variables|SetInstigator _asbp_laser_tank)
      (Variables|Variables|SetGunData (Class|LaserTank|GetGunData _asbp_laser_tank))
      (bind _asgsbp_space_invaders_24 (Utilities|Casting|CastToGSBP_SpaceInvaders24 (Game|GetGameState) :!label _label)
        (:then
          (if (.ReturnValue (Utilities|Map|Find (Variables|/Script/SpaceInvaders24.GS_SpaceInvaders24|GetShotsClasses _asgsbp_space_invaders_24) (Utilities|Array|Get(acopy) (.AvailableShotTypes (Utilities|Struct|BreakGunData (Variables|Variables|GetGunData))) (Math|Random|RandomInteger (Utilities|Array|Length (.AvailableShotTypes (Utilities|Struct|BreakGunData (Variables|Variables|GetGunData))))))))
            (bind _returnvalue_2 (Game|SpawnActorfromClass (.Value (Utilities|Map|Find (Variables|/Script/SpaceInvaders24.GS_SpaceInvaders24|GetShotsClasses _asgsbp_space_invaders_24) (Utilities|Array|Get(acopy) (.AvailableShotTypes (Utilities|Struct|BreakGunData (Variables|Variables|GetGunData))) (Math|Random|RandomInteger (Utilities|Array|Length (.AvailableShotTypes (Utilities|Struct|BreakGunData (Variables|Variables|GetGunData)))))))) (Math|Transform|MakeTransform (Class|GSSpaceInvaders24|TexeltoWorldPos _asgsbp_space_invaders_24 (+ (.Offset (Utilities|Struct|BreakGunData (Variables|Variables|GetGunData))) (Class|ActorinTexels|GetIntTexelPosition (Variables|Variables|GetInstigator)))) (Class|GSSpaceInvaders24|GetGameObjectOrientation _asgsbp_space_invaders_24)) "AlwaysSpawn" "MultiplyWithRoot" 0 (GameplayEffects|MakeOutgoingSpec :self (Variables|Variables|GetASC) :GameplayEffectClass "/Game/Blueprints/GAS/Effects/GE_MakeDamage.GE_MakeDamage_C") (Variables|Variables|GetInstigator)))
            (Utilities|IsValid _returnvalue_2 ; If I don't add this node (that seems obvius), sometimes I get error logs\nThe reason: Shot can dissapear inmediatly after spawn it if is in front of an objective or bunker
              (:Is%20Valid
                (Class|ActorinTexels|SetTexelVelocity _returnvalue_2 (Math|Vector2D|MakeVector2D 0.0 (* (.MovementSpeed (Utilities|GetClassDefaults (.Value (Utilities|Map|Find (Variables|/Script/SpaceInvaders24.GS_SpaceInvaders24|GetShotsClasses _asgsbp_space_invaders_24) (Utilities|Array|Get(acopy) (.AvailableShotTypes (Utilities|Struct|BreakGunData (Variables|Variables|GetGunData))) (Math|Random|RandomInteger (Utilities|Array|Length (.AvailableShotTypes (Utilities|Struct|BreakGunData (Variables|Variables|GetGunData)))))))))) (select (.FromUpToDown (Utilities|Struct|BreakGunData (Variables|Variables|GetGunData))) 1.0 -1.0) 6e+01)))
                (Ability|EndAbility))
              (:Is%20Not%20Valid
                (Ability|CancelAbility :!label _label_2)))
            (else
              (goto _label_2))))
        (:CastFailed
          (goto _label_2))))
    (:CastFailed
      (bind _asenemy (Utilities|Casting|CastToEnemy _returnvalue)
        (:then
          (Variables|Variables|SetASC (Class|Enemy|GetCustomAbilitySystemComponent _asenemy))
          (Variables|Variables|SetInstigator _asenemy)
          (Variables|Variables|SetGunData (Class|Enemy|GetGunData _asenemy))
          (goto _label))
        (:CastFailed
          (goto _label_2))))))

(fn K2CanActivateAbility
  (params (ActorInfo :type Gameplay%20Ability%20Actor%20Info%20Structure) (Handle :type Gameplay%20Ability%20Spec%20Handle%20Structure))
  (bind _avataractor (Utilities|Struct|BreakGameplayAbilityActorInfo ActorInfo))
  (bind _asbp_laser_tank (Utilities|Casting|CastToBP_LaserTank _avataractor)
    (:then
      (return "" (Class|LaserTank|CanShot _asbp_laser_tank)))
    (:CastFailed
      (return "" (.bSuccess (Utilities|Casting|CastToEnemy _avataractor))))))