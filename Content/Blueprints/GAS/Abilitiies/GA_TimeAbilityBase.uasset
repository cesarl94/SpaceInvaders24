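; Base gameplay ability for time powers in Space Invaders 24, which switches the game state in exchange for the laser tank's crystals.
; Activation requires a BP_LaserTank avatar, forward-playing game state and enough Crystals to meet RequiredCrystals.
; On commit it deducts the crystals through the custom ability system component's enum-based attributes, then sets the game state to NewGameState and ends immediately.
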(event Ability|EventActivateAbility
  (Ability|CommitAbility)
  (bind _asgsbp_space_invaders_24 (Utilities|Casting|CastToGSBP_SpaceInvaders24 (Game|GetGameState)))
  (Class|GSSpaceInvaders24|SetNewState _asgsbp_space_invaders_24 (Variables|SpaceInvaders24:TimeAbilityBase|GetNewGameState))
  (Ability|EndAbility))

(event Ability|EventCommitExecute
  (bind _asbp_laser_tank (Utilities|Casting|CastToBP_LaserTank (Ability|GetAvatarActorfromActorInfo))
    (:then
      (Class|CustomAbilitySystemComponent|SetAttributeValuebyEnum (Class|LaserTank|GetCustomAbilitySystemComponent _asbp_laser_tank) "Crystals" (- (Class|CustomAbilitySystemComponent|GetAttributeValuebyEnum (Class|LaserTank|GetCustomAbilitySystemComponent _asbp_laser_tank) "Crystals") (Variables|SpaceInvaders24:TimeAbilityBase|GetRequiredCrystals))))
    (:CastFailed
      (Ability|CancelAbility))))

(fn K2CanActivateAbility
  (params (ActorInfo :type Gameplay%20Ability%20Actor%20Info%20Structure) (Handle :type Gameplay%20Ability%20Spec%20Handle%20Structure))
  (bind (_avataractor _abilitysystemcomponent) (Utilities|Struct|BreakGameplayAbilityActorInfo ActorInfo))
  (Utilities|Casting|CastToBP_LaserTank _avataractor
    (:then
      (bind _ascustom_ability_system_component (Utilities|Casting|CastToCustomAbilitySystemComponent _abilitysystemcomponent)
        (:then
          (bind _asgsbp_space_invaders_24 (Utilities|Casting|CastToGSBP_SpaceInvaders24 (Class|CustomAbilitySystemComponent|GetGameState _ascustom_ability_system_component))
            (:then
              (if (Utilities|Enum|Equal(Enum) (Class|GSSpaceInvaders24|GetGameState _asgsbp_space_invaders_24) (Utilities|Enum|LiteralenumEGameState "PLAYING_FORWARD"))
                (return "" (>= (Math|Float|Round (Class|CustomAbilitySystemComponent|GetAttributeValuebyEnum _ascustom_ability_system_component "Crystals")) (Variables|SpaceInvaders24:TimeAbilityBase|GetRequiredCrystals)))
                (else
                  _)))
            (:CastFailed
              _)))
        (:CastFailed
          _)))
    (:CastFailed
      _))
  (return "" false))