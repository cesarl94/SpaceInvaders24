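; Base Gameplay Ability for time powers that switch the Space Invaders game state in exchange for the laser tank's Crystals.
; Two maps keyed by AbilityInputID supply each ability's crystal cost and target state.
; Activation requires a laser tank with both entries and enough rounded Crystals.
; CommitExecute deducts the cost directly from the attribute, then activation sets the game state and ends immediately.
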(event Ability|EventActivateAbility
  (Ability|CommitAbility)
  (bind _asgsbp_space_invaders_24 (Utilities|Casting|CastToGSBP_SpaceInvaders24 (Game|GetGameState)))
  (Class|GSSpaceInvaders24|SetNewState _asgsbp_space_invaders_24 (.Value (Utilities|Map|Find (Variables|Default|GetGameStateByAbility) (Variables|Default|GetAbilityInputID))))
  (Ability|EndAbility))

(event Ability|EventCommitExecute
  (bind _cristalsbyability (Variables|Default|GetCristalsByAbility))
  (bind _abilityinputid (Variables|Default|GetAbilityInputID))
  (bind (_value _returnvalue) (Utilities|Map|Find _cristalsbyability _abilityinputid))
  (bind _asbp_laser_tank (Utilities|Casting|CastToBP_LaserTank (Ability|GetAvatarActorfromActorInfo))
    (:then
      (if _returnvalue
        (Class|CustomAbilitySystemComponent|SetAttributeValuebyEnum (Class|LaserTank|GetCustomAbilitySystemComponent _asbp_laser_tank) "Crystals" (- (Class|CustomAbilitySystemComponent|GetAttributeValuebyEnum (Class|LaserTank|GetCustomAbilitySystemComponent _asbp_laser_tank) "Crystals") _value))
        (else
          (Ability|CancelAbility :!label _label))))
    (:CastFailed
      (goto _label))))

(fn K2CanActivateAbility
  (params (ActorInfo :type Gameplay%20Ability%20Actor%20Info%20Structure) (Handle :type Gameplay%20Ability%20Spec%20Handle%20Structure))
  (bind (_owneractor _avataractor _playercontroller _abilitysystemcomponent) (Utilities|Struct|BreakGameplayAbilityActorInfo ActorInfo))
  (bind _cristalsbyability (Variables|Default|GetCristalsByAbility))
  (bind _abilityinputid (Variables|Default|GetAbilityInputID))
  (bind (_value _returnvalue) (Utilities|Map|Find _cristalsbyability _abilityinputid))
  (Utilities|Casting|CastToBP_LaserTank _avataractor
    (:then
      (bind _ascustom_ability_system_component (Utilities|Casting|CastToCustomAbilitySystemComponent _abilitysystemcomponent)
        (:then
          (if (and _returnvalue (.ReturnValue (Utilities|Map|Find (Variables|Default|GetGameStateByAbility) (Variables|Default|GetAbilityInputID))))
            (return "" (>= (Math|Float|Round (Class|CustomAbilitySystemComponent|GetAttributeValuebyEnum _ascustom_ability_system_component "Crystals")) _value))
            (else
              _)))
        (:CastFailed
          _)))
    (:CastFailed
      _))
  (return "" false))