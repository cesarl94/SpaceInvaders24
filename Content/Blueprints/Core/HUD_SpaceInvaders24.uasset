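; HUD class for the Space Invaders game that creates and displays the main UI widget.
; On BeginPlay it shows the mouse cursor, then creates WBP_Main for the owning player and adds it to the viewport.
; Every Tick it compares the viewport size with a cached value and passes any change to the widget's resize handler, WBPMainOnResize.
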(event Custom|#HUD%20CheckScreenSize
  (bind _returnvalue (Viewport|GetViewportSize))
  (if (Utilities|Operators|NotEqual(!=) (Variables|Default|GetScreenSize) _returnvalue 0.0)
    (bind _output_get (Variables|Default|SetScreenSize _returnvalue))
    (Default|WBPMainonResize (Variables|Default|GetUI) (.x _output_get) (.y _output_get))))

(event EventBeginPlay
  (bind _returnvalue (Game|Player|GetOwningPlayerController))
  (Variables|/Script/Engine.PlayerController|SetbShowMouseCursor _returnvalue true)
  (bind _returnvalue_2 (UserInterface|CreateWidget "/Game/Blueprints/UI/WBP_Main.WBP_Main_C" _returnvalue))
  (bind _output_get (Variables|Default|SetUI _returnvalue_2))
  (UserInterface|Viewport|AddtoViewport _output_get 0))

(event EventTick
  (params (DeltaSeconds :type Float%20%28single-precision%29))
  (CallFunction|#HUDCheckScreenSize))

(fn ConstructionScript)