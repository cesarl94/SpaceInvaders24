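; Player controller for a Space Invaders-style game that routes input to the player's laser tank.
; Each input event casts the controlled pawn to BP_LaserTank and does nothing if the cast fails.
; The horizontal axis sets tank movement, the shoot action fires, and three skill actions trigger skills by slot index.
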(event Input|ActionEvents|InputActionEscape
  (params (Key :type Key%20Structure :default "None")))

(event Input|ActionEvents|InputActionEnter
  (params (Key :type Key%20Structure :default "None")))

(event Input|ActionEvents|InputActionShoot
  (params (Key :type Key%20Structure :default "None"))
  (:Pressed
    (bind _asbp_laser_tank (Utilities|Casting|CastToBP_LaserTank (Pawn|GetControlledPawn)))
    (Default|LaserTankShoot _asbp_laser_tank)))

(event Input|ActionEvents|InputActionSkill1
  (params (Key :type Key%20Structure :default "None"))
  (:Pressed
    (bind _asbp_laser_tank (Utilities|Casting|CastToBP_LaserTank (Pawn|GetControlledPawn)))
    (Default|LaserTankInputSkill _asbp_laser_tank)))

(event Input|ActionEvents|InputActionSkill2
  (params (Key :type Key%20Structure :default "None"))
  (:Pressed
    (bind _asbp_laser_tank (Utilities|Casting|CastToBP_LaserTank (Pawn|GetControlledPawn)))
    (Default|LaserTankInputSkill _asbp_laser_tank 1)))

(event Input|ActionEvents|InputActionSkill3
  (params (Key :type Key%20Structure :default "None"))
  (:Pressed
    (bind _asbp_laser_tank (Utilities|Casting|CastToBP_LaserTank (Pawn|GetControlledPawn)))
    (Default|LaserTankInputSkill _asbp_laser_tank 2)))

(event Input|AxisEvents|InputAxisMoveHorizontal
  (params (AxisValue :type Float%20%28single-precision%29))
  (bind _asbp_laser_tank (Utilities|Casting|CastToBP_LaserTank (Pawn|GetControlledPawn)))
  (Class|LaserTank|SetHorizontalMovement _asbp_laser_tank AxisValue))

(fn ConstructionScript)